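; BP_WildGrass is a wild grass weed actor for the farming simulator's gardening components.
; Its construction script picks a random grass mesh variant, then line-traces straight down on TraceTypeQuery3 from the mesh's location.
; A hit snaps the actor to the impact point, and a miss destroys it.
; The event graph holds only disabled stub events, so this Blueprint adds no runtime logic of its own.
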(event EventBeginPlay
  (|CallParentFunction) ; This node is disabled and will not be called.\nDrag off pins to build functionality.
)

(event Collision|EventActorBeginOverlap
  (params (OtherActor :type Actor%20Object%20Reference))
  (|CallParentFunction OtherActor) ; This node is disabled and will not be called.\nDrag off pins to build functionality.
)

(event EventTick
  (params (DeltaSeconds :type Float%20%28single-precision%29))
  (|CallParentFunction DeltaSeconds) ; This node is disabled and will not be called.\nDrag off pins to build functionality.
)

(fn ConstructionScript
  (bind _staticmesh (Variables|Default|GetStaticMesh))
  (bind _returnvalue (Transformation|GetWorldLocation _staticmesh))
  (|CallParentFunction)
  (Components|StaticMesh|SetStaticMesh (Variables|Default|GetStaticMesh) (.OutItem (Utilities|Array|Random (Utilities|Array|MakeArray "/Game/FarmingSimulator/GameAssets/Weeds/Wild_Grass_vlkhcbxia_High_vlkhcbxia_VarA_LOD0.Wild_Grass_vlkhcbxia_High_vlkhcbxia_VarA_LOD0" "/Game/FarmingSimulator/GameAssets/Weeds/Wild_Grass_vlkhcbxia_High_vlkhcbxia_VarA_LOD1.Wild_Grass_vlkhcbxia_High_vlkhcbxia_VarA_LOD1" "/Game/FarmingSimulator/GameAssets/Weeds/Wild_Grass_vlkhcbxia_High_vlkhcbxia_VarA_LOD2.Wild_Grass_vlkhcbxia_High_vlkhcbxia_VarA_LOD2" "/Game/FarmingSimulator/GameAssets/Weeds/Wild_Grass_vlkhcbxia_High_vlkhcbxia_VarC_LOD2.Wild_Grass_vlkhcbxia_High_vlkhcbxia_VarC_LOD2"))))
  (bind (_outhit _returnvalue_2) (Collision|LineTraceByChannel _returnvalue (- _returnvalue "0.000000,0.000000,10000.000000") "TraceTypeQuery3" false 0 "None"))
  (if _returnvalue_2
    (Transformation|SetActorLocation (.Location (Collision|BreakHitResult _outhit)) false false)
    (else
      (Actor|DestroyActor))))