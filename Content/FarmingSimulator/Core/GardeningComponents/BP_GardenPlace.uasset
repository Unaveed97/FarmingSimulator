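; Garden plot actor for the farming game that tracks its plants, removes overlapping foliage instances and shows a grow-time countdown in 3D text.
; A looping timer randomly spawns weeds while plants exist, lowering every plant's growth factor and adjusting its health per tick.
; Weed spots are random points in the box, with recursive retries on a plant proximity check.
; Destroy handlers restore growth factor, adjust health again and drop collected plants.
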(event OnComponentBeginOverlap(Box)
  (params (OverlappedComponent :type Primitive%20Component%20Object%20Reference) (OtherActor :type Actor%20Object%20Reference) (OtherComp :type Primitive%20Component%20Object%20Reference) (OtherBodyIndex :type Integer) (bFromSweep :type Boolean) (SweepResult :type Hit%20Result%20Structure%20%28by%20ref%29))
  (bind _asfoliage_instanced_static_mesh_component (Utilities|Casting|CastToFoliageInstancedStaticMeshComponent OtherComp))
  (CallFunction|RemoveFoliage _asfoliage_instanced_static_mesh_component OtherBodyIndex))

(event EventBeginPlay
  (bind _asbp_third_person_character (Utilities|Casting|CastToBP_ThirdPersonCharacter (Game|GetPlayerCharacter 0)))
  (Utilities|IsValid _asbp_third_person_character
    (:Is%20Valid
      (Variables|References|SetCharacter_Ref _asbp_third_person_character)
      (bind _aspc_farming_simulator (Utilities|Casting|CastToPC_FarmingSimulator (Game|GetPlayerController 0)))
      (Utilities|IsValid _aspc_farming_simulator
        (:Is%20Valid
          (Variables|References|SetController_Ref _aspc_farming_simulator)
          (Variables|/Script/Text3D.Text3DComponent|SetText (Variables|Default|GetText3D) (Variables|Default|GetValue))
          (Utilities|Time|SetTimerbyFunctionName 0 "WeedsLoop" 15.0 true))))))

(fn ConstructionScript)

(fn AddPlant
  (params (Plants :type BP%20Plant%20Parent%20Object%20Reference%20%28by%20ref%29))
  (Game|BindEventtoOnDestroyed (EventDispatchers|CreateEvent :!event OnPlantCollected))
  (Utilities|Array|Add (Variables|Default|GetPlants) Plants))

(fn WeedsLoop
  (if (not (Utilities|Array|IsEmpty (Variables|Default|GetPlants)))
    (if (< (Math|Random|RandomFloatinRange 0.0 1e+02) (Variables|Weeds|GetWeedSpawnChance))
      (bind (_transform _success) (CallFunction|GenerateWeedTransform))
      (if _success
        (bind _returnvalue (Game|SpawnActorfromClass "/Game/FarmingSimulator/Core/GardeningComponents/Weeds/BP_WildGrass.BP_WildGrass_C" _transform "Undefined" "MultiplyWithRoot" 0 0))
        (Game|BindEventtoOnDestroyed _returnvalue (EventDispatchers|CreateEvent :!event OnWeedDestroyed))
        (for _array_element (Variables|Default|GetPlants)
          (Variables|/Game/FarmingSimulator/Core/GardeningComponents/Plants/BP_PlantParent.BP_PlantParent_C|SetGrowthFactor _array_element (Math|Float|Clamp(Float) (- (Variables|/Game/FarmingSimulator/Core/GardeningComponents/Plants/BP_PlantParent.BP_PlantParent_C|GetGrowthFactor _array_element) (Variables|/Game/FarmingSimulator/Core/GardeningComponents/Weeds/BP_Weed.BP_Weed_C|GetGrowSpeedDamage _returnvalue)) 0.1))
          (Variables|/Game/FarmingSimulator/Core/GardeningComponents/Plants/BP_PlantParent.BP_PlantParent_C|SetPlantHealthPerGrowTick _array_element (+ (Variables|/Game/FarmingSimulator/Core/GardeningComponents/Weeds/BP_Weed.BP_Weed_C|GetHealthDamage _returnvalue) (Variables|/Game/FarmingSimulator/Core/GardeningComponents/Plants/BP_PlantParent.BP_PlantParent_C|GetPlantHealthPerGrowTick _array_element))))))))

(fn GenerateWeedTransform
  (params (Attempt :type Integer))
  (bind _returnvalue (Math|Random|RandomFloatinRange 1.0 2.5))
  (bind _returnvalue_2 (Transformation|GetActorLocation))
  (bind _box (Variables|Default|GetBox))
  (bind _returnvalue_3 (Components|Box|GetScaledBoxExtent _box))
  (bind _returnvalue_4 (+ (.z _returnvalue_2) 1e+03))
  (bind (_x _y) (Math|Vector|BreakVector _returnvalue_3))
  (bind _returnvalue_5 (* _y -1.0))
  (bind _returnvalue_6 (* _x -1.0))
  (bind _returnvalue_7 (Math|Random|RandomFloatinRange _returnvalue_5 _y))
  (bind _returnvalue_8 (Math|Random|RandomFloatinRange _returnvalue_6 _x))
  (bind _returnvalue_9 (+ (.x _returnvalue_2) _returnvalue_8))
  (bind _returnvalue_10 (+ (.y _returnvalue_2) _returnvalue_7))
  (bind _returnvalue_11 (Math|Vector|MakeVector _returnvalue_9 _returnvalue_10 _returnvalue_4))
  (if (< Attempt 10)
    (bind _array_element (Utilities|Array|ForEachLoopwithBreak (Variables|Default|GetPlants) :!label _label)
      (:LoopBody
        (if (< (Math|Vector|Distance(Vector) (Transformation|GetActorLocation _array_element) _returnvalue_11) 5e+01)
          (LocalVariables|SetShouldRegenarate true)
          (goto _label Break)))
      (:Completed
        (if (LocalVariables|GetShouldRegenarate)
          (bind (_transform _success) (CallFunction|GenerateWeedTransform (+ Attempt 1)))
          (return _transform _success)
          (else
            (return (Math|Transform|MakeTransform _returnvalue_11 (Math|Rotator|MakeRotator 0.0 0.0 (Math|Random|RandomFloatinRange 0.0 3.6e+02)) (Math|Vector|MakeVector _returnvalue _returnvalue _returnvalue)) true)))))
    (else
      (return "" false))))

(fn OnWeedDestroyed
  (params (Weed :type Actor%20Object%20Reference))
  (bind _asbp_weed (Utilities|Casting|CastToBP_Weed Weed))
  (for _array_element (Variables|Default|GetPlants)
    (Variables|/Game/FarmingSimulator/Core/GardeningComponents/Plants/BP_PlantParent.BP_PlantParent_C|SetGrowthFactor _array_element (Math|Float|Clamp(Float) (+ (Variables|/Game/FarmingSimulator/Core/GardeningComponents/Plants/BP_PlantParent.BP_PlantParent_C|GetGrowthFactor _array_element) (Variables|/Game/FarmingSimulator/Core/GardeningComponents/Weeds/BP_Weed.BP_Weed_C|GetGrowSpeedDamage _asbp_weed)) 0.1))
    (Variables|/Game/FarmingSimulator/Core/GardeningComponents/Plants/BP_PlantParent.BP_PlantParent_C|SetPlantHealthPerGrowTick _array_element (+ (Variables|/Game/FarmingSimulator/Core/GardeningComponents/Weeds/BP_Weed.BP_Weed_C|GetHealthDamage _asbp_weed) (Variables|/Game/FarmingSimulator/Core/GardeningComponents/Plants/BP_PlantParent.BP_PlantParent_C|GetPlantHealthPerGrowTick _array_element)))))

(fn OnPlantCollected
  (params (DestroyedActor :type Actor%20Object%20Reference))
  (bind _asbp_plant_parent (Utilities|Casting|CastToBP_PlantParent DestroyedActor))
  (Utilities|Array|RemoveItem (Variables|Default|GetPlants) _asbp_plant_parent))

(fn RemoveFoliage
  (params (InstanceComponent :type Foliage%20Instanced%20Static%20Mesh%20Component%20Object%20Reference) (Index :type Integer))
  (Class|InstancedStaticMeshComponent|RemoveInstance InstanceComponent Index))