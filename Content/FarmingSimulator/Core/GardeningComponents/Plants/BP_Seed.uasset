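; BP_Seed is a wheat seed pickup in the farming simulator that the player collects by walking into it.
; On BeginPlay it caches the PC_FarmingSimulator player controller.
; When the third-person character overlaps its box, it increments the controller's wheat seed count, prints the new total, destroys itself and sets the controller's HasSeed flag.
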(event OnComponentBeginOverlap(Box)
  (params (OverlappedComponent :type Primitive%20Component%20Object%20Reference) (OtherActor :type Actor%20Object%20Reference) (OtherComp :type Primitive%20Component%20Object%20Reference) (OtherBodyIndex :type Integer) (bFromSweep :type Boolean) (SweepResult :type Hit%20Result%20Structure%20%28by%20ref%29))
  (bind _controller_ref (Variables|Default|GetController_ref))
  (Utilities|Casting|CastToBP_ThirdPersonCharacter OtherActor)
  (bind _result (Math|Integer|IncrementInt (Variables|/Game/FarmingSimulator/Core/PC_FarmingSimulator.PC_FarmingSimulator_C|GetAmountOfWheatSeeds _controller_ref))
    (:%20%20
      (bind _output_get (Variables|/Game/FarmingSimulator/Core/PC_FarmingSimulator.PC_FarmingSimulator_C|SetAmountOfWheatSeeds _controller_ref _result))
      (Development|PrintString (Utilities|String|Append "number seed " (Utilities|String|ToString(Integer) _output_get)))
      (Actor|DestroyActor)
      (Variables|/Game/FarmingSimulator/Core/PC_FarmingSimulator.PC_FarmingSimulator_C|SetHasSeed? (Variables|Default|GetController_ref) true))))

(event EventBeginPlay
  (bind _aspc_farming_simulator (Utilities|Casting|CastToPC_FarmingSimulator (Game|GetPlayerController 0)))
  (Utilities|IsValid _aspc_farming_simulator
    (:Is%20Valid
      (Variables|Default|SetController_ref _aspc_farming_simulator))))

(fn ConstructionScript)