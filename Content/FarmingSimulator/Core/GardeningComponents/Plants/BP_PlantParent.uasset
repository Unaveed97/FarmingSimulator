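; Parent actor for farm plants that grow over time and are harvested as "Tomatos" into the player controller's inventory.
; A data table row supplies growth stages, speed and yield, with the mesh and scale taken from the stage nearest current progress.
; A looping timer advances growth, drains health and recalculates fruit from both.
; Preview functions swap materials for placement validity, and interaction past a growth threshold harvests and destroys the plant.
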(event OnInteracted(BPC_InteractableComponent)
  (CallFunction|OnPickup))

(event Custom|GatherPlant_Server
  (CallFunction|GatherPlantClient))

(event Custom|GatherPlant_Client)

(event EventBeginPlay
  (bind _aspc_farming_simulator (Utilities|Casting|CastToPC_FarmingSimulator (Game|GetPlayerController 0)))
  (Utilities|IsValid _aspc_farming_simulator
    (:Is%20Valid
      (Variables|Default|SetController_Ref _aspc_farming_simulator)
      (bind _asgm_state_farming (Utilities|Casting|CastToGM_State_Farming (Game|GetGameState)))
      (Utilities|IsValid _asgm_state_farming
        (:Is%20Valid
          (Variables|Default|SetGM_State_Ref _asgm_state_farming))))))

(event EventTick
  (params (DeltaSeconds :type Float%20%28single-precision%29))
  (CallFunction|CanInteract))

(event EventOnPickup
  (bind _amountoffruitgathered (Variables|Default|GetAmountOfFruitGathered))
  (bind _can_ (CallFunction|CanInteract))
  (if _can_
    (Development|PrintString (Utilities|String|Append "Hi i picked : " " ; " (Utilities|String|ToString(Integer) _amountoffruitgathered) "Tomatos"))
    (Default|AddtoInventory (Variables|/Game/FarmingSimulator/Core/PC_FarmingSimulator.PC_FarmingSimulator_C|GetBPC_Inventory (Variables|Default|GetController_Ref)) "Tomatos" _amountoffruitgathered)
    (Actor|DestroyActor)))

(fn ConstructionScript
  (bind _plantinforowhandle (Variables|Default|GetPlantInfoRowHandle))
  (bind (_datatable _rowname) (Utilities|Struct|BreakDataTableRowHandle _plantinforowhandle))
  (bind _returnvalue (Utilities|GetDataTableRow _datatable _rowname)
    (:then
      (Variables|PlantAttributes|SetS_PlantInfo _returnvalue)
      (CallFunction|UpdatewithProgress))))

(fn StartPreviewing
  (Collision|SetCollisionEnabled (Variables|Default|GetInteractionBox) "NoCollision")
  (bind _output_get (Variables|Default|SetBaseMaterials (Rendering|Material|GetMaterials (Variables|Default|GetStaticMesh))))
  (for (_ _array_index) _output_get
    (Rendering|Material|SetMaterial (Variables|Default|GetStaticMesh) _array_index "/Game/FarmingSimulator/Core/GardeningComponents/Plants/M_PlantPreview.M_PlantPreview")
    (Variables|Default|SetIsPreviewing? true)))

(fn SetIsValid
  (params (IsValid :type Boolean))
  (if (!= IsValid (Variables|Default|GetPreviousIsValid?))
    (if (Variables|Default|GetIsPreviewing?)
      (for (_ _array_index) (Variables|Default|GetBaseMaterials)
        (Rendering|Material|SetMaterial (Variables|Default|GetStaticMesh) _array_index (select IsValid "/Game/FarmingSimulator/Core/GardeningComponents/Plants/M_PlantPreview.M_PlantPreview" "/Game/FarmingSimulator/Core/GardeningComponents/Plants/MI_PlantMaterialRed.MI_PlantMaterialRed")))
      (Variables|Default|SetPreviousIsValid? IsValid))))

(fn Plant
  (Utilities|Time|SetTimerbyFunctionName 0 "GrowLoop" 15.0 true))

(fn FindGrowthState
  (params (Progress :type Float%20%28double-precision%29))
  (bind _s_plantinfo (Variables|PlantAttributes|GetS_PlantInfo))
  (bind _growthinfo (Utilities|Struct|BreakS_Plants _s_plantinfo))
  (bind _output (Utilities|Array|Get(acopy) _growthinfo))
  (LocalVariables|SetMinProgress (.GrowthProgress (Utilities|Struct|BreakS_PlantGrowthState _output)))
  (LocalVariables|SetMinState _output)
  (for _array_element _growthinfo
    (if (< (Math|Float|Absolute(Float) (- (.GrowthProgress (Utilities|Struct|BreakS_PlantGrowthState _array_element)) Progress)) (Math|Float|Absolute(Float) (- (LocalVariables|GetMinProgress) Progress)))
      (LocalVariables|SetMinState _array_element)
      (LocalVariables|SetMinProgress (.GrowthProgress (Utilities|Struct|BreakS_PlantGrowthState _array_element)))))
  (return (LocalVariables|GetMinState)))

(fn UpdatewithProgress
  (bind _growstate (CallFunction|FindGrowthState (Variables|PlantAttributes|GetGrowProgress)))
  (Components|StaticMesh|SetStaticMesh (Variables|Default|GetStaticMesh) (.StaticMesh (Utilities|Struct|BreakS_PlantGrowthState _growstate)))
  (Transformation|SetRelativeScale3D (Variables|Default|GetStaticMesh) (.Scale (Utilities|Struct|BreakS_PlantGrowthState _growstate))))

(fn GrowLoop
  (bind _factor (CallFunction|CountFruitsAmountFactor))
  (bind _s_plantinfo (Variables|PlantAttributes|GetS_PlantInfo))
  (Development|PrintString "Hello i am in grow loop function")
  (if (<= (Variables|PlantAttributes|GetGrowProgress) 1.0)
    (Variables|PlantAttributes|SetGrowProgress (+ (Variables|PlantAttributes|GetGrowProgress) (* (.GrowSpeed (Utilities|Struct|BreakS_Plants (Variables|PlantAttributes|GetS_PlantInfo))) (Variables|Default|GetGrowthFactor))))
    (CallFunction|UpdatewithProgress)
    (Variables|PlantAttributes|SetPlantHealth (- (Variables|PlantAttributes|GetPlantHealth) (Variables|PlantAttributes|GetPlantHealthPerGrowTick)))
    (Utilities|FlowControl|Sequence
      (:then_0
        (if (.israndomlygenerated _s_plantinfo)
          (Variables|PlantAttributes|SetAmountOfFruit (Math|Float|Truncate (* (Math|Random|RandomIntegerinRange (.amountrangemin _s_plantinfo) (.amountrangemax _s_plantinfo)) _factor)))
          (else
            (Variables|PlantAttributes|SetAmountOfFruit (Math|Float|Truncate (* (.amountoffruit _s_plantinfo) _factor))))))
      (:then_1
        (Development|PrintString (Utilities|String|Append "Hi I have Gathered  " ": " (Utilities|String|ToString(Integer) (Variables|PlantAttributes|GetAmountOfFruit))))
        (Variables|Default|SetAmountOfFruitGathered (Variables|PlantAttributes|GetAmountOfFruit))))))

(fn CountFruitsAmountFactor
  (bind _planthealth (Variables|PlantAttributes|GetPlantHealth))
  (bind _returnvalue (/ _planthealth 1e+02))
  (Utilities|FlowControl|Sequence
    (:then_0
      (if (Math|Float|InRange(Float) (Variables|PlantAttributes|GetGrowProgress) 0.0 0.5)
        (bind _output_get (LocalVariables|SetDefaultFactor (/ (Variables|PlantAttributes|GetGrowProgress) 3.0)))
        (LocalVariables|SetDefaultFactor (* _output_get _returnvalue))
        (else
          (bind _output_get_2 (LocalVariables|SetDefaultFactor (* (LocalVariables|GetDefaultFactor) (Variables|PlantAttributes|GetGrowProgress))))
          (LocalVariables|SetDefaultFactor (* _returnvalue _output_get_2)))))
    (:then_1
      (return (LocalVariables|GetDefaultFactor)))))

(fn CanInteract
  (return (> (Variables|PlantAttributes|GetGrowProgress) 0.3)))