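; BP_Item is a farming tool pickup that can till the landscape when used as a hoe.
; Construction applies the chosen mesh; interacting calls the controller's PickUpTool, disables further interaction and removes the widget reference created on BeginPlay.
; On attack, if the Arrow carries the hoe tag, it traces down, then up as fallback, spawning BP_GardenPlace on near-flat Landscape hits.
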(event OnInteracted(BPC_InteractableComponent)
  (CallFunction|PickUp))

(event EventPickUp
  (Development|PrintString "Hello i tried to pickup item")
  (Default|PickUpTool (Variables|Default|GetController_Ref))
  (Default|EnableInteractions (Variables|Default|GetBPC_InteractableComponent) false)
  (Development|PrintString "Item Picked")
  (Utilities|FlowControl|DelayUntilNextTick)
  (Widget|RemovefromParent (Variables|Default|GetInteractWidget_Ref)))

(event EventBeginPlay
  (bind _returnvalue (UserInterface|CreateWidget "/Game/FarmingSimulator/Widgets/WBP_Interact.WBP_Interact_C"))
  (Variables|Default|SetInteractWidget_Ref _returnvalue)
  (bind _aspc_farming_simulator (Utilities|Casting|CastToPC_FarmingSimulator (Game|GetPlayerController 0)))
  (Utilities|IsValid _aspc_farming_simulator
    (:Is%20Valid
      (Variables|Default|SetController_Ref _aspc_farming_simulator)
      (bind _asgm_state_farming (Utilities|Casting|CastToGM_State_Farming (Game|GetGameState)))
      (Utilities|IsValid _asgm_state_farming
        (:Is%20Valid
          (Variables|Default|SetGameState_Ref _asgm_state_farming)
          (bind _asbp_third_person_character (Utilities|Casting|CastToBP_ThirdPersonCharacter (Game|GetPlayerCharacter 0)))
          (Utilities|IsValid _asbp_third_person_character
            (:Is%20Valid
              (Variables|Default|SetCharacterRef _asbp_third_person_character))))))))

(event EventOnAttackPressed
  (Development|PrintString "I was Called")
  (CallFunction|TraceonAttack))

(fn ConstructionScript
  (Components|StaticMesh|SetStaticMesh (Variables|Default|GetItemModel) (Variables|Default|GetItemToPickUp)))

(fn TraceonAttack
  (bind _arrow (Variables|Default|GetArrow))
  (bind _returnvalue (Transformation|GetWorldLocation _arrow))
  (Utilities|FlowControl|Sequence
    (:then_0
      ;[0.15 0.15 0.15 0.5] LineTrace
      (if (Components|ComponentHasTag _arrow "HoeLineTraceLocation")
        (bind (_outhit _returnvalue_2) (Collision|LineTraceByChannel _returnvalue (+ _returnvalue (Math|Vector|MakeVector 0.0 0.0 -3e+02)) "TraceTypeQuery1" false 0 "None"))
        (if _returnvalue_2
          (Variables|Default|SetLocalHitResult _outhit)
          (Variables|Default|SetHit? true)
          (else
            (bind (_outhit_2 _returnvalue_3) (Collision|LineTraceByChannel _returnvalue (+ _returnvalue (Math|Vector|MakeVector 0.0 0.0 3e+02)) "TraceTypeQuery1" false 0 "None"))
            (if _returnvalue_3
              (Variables|Default|SetLocalHitResult _outhit_2)
              (Variables|Default|SetHit? true))))))
    (:then_1
      (if (Variables|Default|GetHit?)
        (Utilities|Casting|CastToLandscape (.HitActor (Collision|BreakHitResult (Variables|Default|GetLocalHitResult))))
        (if (and (Math|Float|InRange(Float) (.X (Math|Vector|BreakVector (.Normal (Collision|BreakHitResult (Variables|Default|GetLocalHitResult))))) -0.15 0.15) (Math|Float|InRange(Float) (.Y (Math|Vector|BreakVector (.Normal (Collision|BreakHitResult (Variables|Default|GetLocalHitResult))))) -0.15 0.15))
          (Game|SpawnActorfromClass "/Game/FarmingSimulator/Core/GardeningComponents/BP_GardenPlace.BP_GardenPlace_C" (Math|Transform|MakeTransform (.Location (Collision|BreakHitResult (Variables|Default|GetLocalHitResult))) "0, 0, 0" "1.000000,1.000000,1.000000") "Undefined" "MultiplyWithRoot" (Variables|Default|GetCharacterRef) 0))))))