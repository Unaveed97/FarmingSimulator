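; BPC_Interaction is a player component that lets the third-person character find and interact with objects in the farming simulator.
; Every tick it line-traces from the follow camera, toggling the interaction widget on each hit actor's BPC_InteractableComponent as the target changes.
; Pressing E calls OnInteract on the last hit actor, which stays stored even after the trace misses and hides its widget.
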(event Custom|InteractWithCurrentObject
  (Default|OnInteract (Actor|GetComponentbyClass (Variables|Default|GetLastInteractionObject) "/Game/FarmingSimulator/Core/InteractionSystem/BPC_InteractableComponent.BPC_InteractableComponent_C")))

(event EventBeginPlay
  (bind _asbp_third_person_character (Utilities|Casting|CastToBP_ThirdPersonCharacter (Components|GetOwner)))
  (Utilities|IsValid _asbp_third_person_character
    (:Is%20Valid
      (Variables|Default|SetCharacter _asbp_third_person_character))))

(event EventTick
  (params (DeltaSeconds :type Float%20%28single-precision%29))
  (CallFunction|MakeTrace))

(event Input|KeyboardEvents|E
  (params (Key :type Key%20Structure :default "None"))
  (:Pressed
    (Variables|Default|GetLastInteractionObject
      (:then
        (CallFunction|InteractwithCurrentObject))
      (:else))))

(fn MakeTrace
  (bind _character (Variables|Default|GetCharacter))
  (bind _followcamera (Variables|/Game/ThirdPerson/Blueprints/BP_ThirdPersonCharacter.BP_ThirdPersonCharacter_C|GetFollowCamera _character))
  (bind _returnvalue (Transformation|GetWorldLocation _followcamera))
  (bind (_outhit _returnvalue_2) (Collision|LineTraceByChannel _returnvalue (+ _returnvalue (* (Math|Vector|GetForwardVector _followcamera) 5e+02)) "TraceTypeQuery4" false 0 "None"))
  (if _returnvalue_2
    (CallFunction|HandleTraceHit _outhit)
    (else
      (bind _lastinteractionobject (Variables|Default|GetLastInteractionObject)
        (:then
          (Default|ShowInteractionWidget (Actor|GetComponentbyClass _lastinteractionobject "/Game/FarmingSimulator/Core/InteractionSystem/BPC_InteractableComponent.BPC_InteractableComponent_C") false))
        (:else)))))

(fn HandleTraceHit
  (params (Hit :type Hit%20Result%20Structure))
  (bind _hitactor (Collision|BreakHitResult Hit))
  (bind _lastinteractionobject (Variables|Default|GetLastInteractionObject)
    (:then
      (if (== _lastinteractionobject _hitactor)
        _
        (else
          (Default|ShowInteractionWidget (Actor|GetComponentbyClass (Variables|Default|GetLastInteractionObject) "/Game/FarmingSimulator/Core/InteractionSystem/BPC_InteractableComponent.BPC_InteractableComponent_C") false)
          (Variables|Default|SetLastInteractionObject _hitactor :!label _label))))
    (:else
      (goto _label)))
  (Default|ShowInteractionWidget (Actor|GetComponentbyClass _hitactor "/Game/FarmingSimulator/Core/InteractionSystem/BPC_InteractableComponent.BPC_InteractableComponent_C") true))