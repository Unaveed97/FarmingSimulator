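; BP_ShopKeeper_Npc is a shopkeeper NPC that opens the shop UI when the player walks into its trigger.
; On BeginPlay it creates a WB_ShopUI widget linked to itself and caches the player controller and character.
; On overlap with the player it shows the cursor, switches to game-and-UI input, disables character movement and adds the widget to the viewport.
; Closing the shop and restoring movement are not handled here.
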(event OnComponentBeginOverlap(ShopTrigger)
  (params (OverlappedComponent :type Primitive%20Component%20Object%20Reference) (OtherActor :type Actor%20Object%20Reference) (OtherComp :type Primitive%20Component%20Object%20Reference) (OtherBodyIndex :type Integer) (bFromSweep :type Boolean) (SweepResult :type Hit%20Result%20Structure%20%28by%20ref%29))
  (bind _controller_ref (Variables|Default|GetController_Ref))
  (if (== OtherActor (Game|GetPlayerCharacter 0))
    (Development|PrintString "Hello I am tring to interact with the shop")
    (Variables|/Script/Engine.PlayerController|SetbShowMouseCursor _controller_ref true)
    (Input|SetInputModeGameandUI _controller_ref (Variables|Default|GetWb_Shop_Ref) "LockOnCapture" false false)
    (Pawn|Components|CharacterMovement|DisableMovement (Variables|/Script/Engine.Character|GetCharacterMovement (Variables|Default|GetCharacterRef)))
    (UserInterface|Viewport|AddtoViewport (Variables|Default|GetWb_Shop_Ref) 0)))

(event EventBeginPlay
  (bind _returnvalue (Game|GetPlayerController 0))
  (bind _aspc_farming_simulator (Utilities|Casting|CastToPC_FarmingSimulator _returnvalue))
  (bind _returnvalue_2 (UserInterface|CreateWidget "/Game/FarmingSimulator/Widgets/ShopUi/WB_ShopUI.WB_ShopUI_C" 0 self))
  (Utilities|IsValid _returnvalue_2
    (:Is%20Valid
      (Variables|Default|SetWb_Shop_Ref _returnvalue_2)
      (Utilities|IsValid _aspc_farming_simulator
        (:Is%20Valid
          (Variables|Default|SetController_Ref _aspc_farming_simulator)
          (bind _asbp_third_person_character (Utilities|Casting|CastToBP_ThirdPersonCharacter (Game|GetPlayerCharacter 0)))
          (Variables|Default|SetCharacterRef _asbp_third_person_character))))))

(fn ConstructionScript)