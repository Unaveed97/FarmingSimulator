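; Player controller for the farming simulator, handling input for planting, hoe tilling and the inventory camera and UI, plus a money-spending helper.
; On BeginPlay it spawns a tomato preview actor into the game state, which a toggled Tick camera trace moves while seeds are held.
; Sowing requires the validation box to overlap only garden plots, then spawns and registers the plant.
; Spawning and tool actions use Server/Client event pairs.
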(event Custom|MeshMovementTrace
  (bind _playercameramanager (Variables|Default|GetPlayerCameraManager))
  (bind _gamestate_ref (Variables|Reference|GetGameState_Ref))
  (bind _transformcomponent (Variables|/Script/Engine.PlayerCameraManager|GetTransformComponent _playercameramanager))
  (bind _plantactor (Variables|/Game/FarmingSimulator/Core/GM_State_Farming.GM_State_Farming_C|GetPlantActor _gamestate_ref))
  (bind _returnvalue (Transformation|GetWorldLocation _transformcomponent))
  ;[0.15 0.15 0.15 0.5] Spawning the plant preview where it can be placed
  (bind (_outhit _returnvalue_2) (Collision|LineTraceByChannel _returnvalue (+ _returnvalue (* (Math|Vector|GetForwardVector _transformcomponent) 1.5e+03)) "TraceTypeQuery3" false 0 "None"))
  (if _returnvalue_2
    (Transformation|SetActorLocation _plantactor (.Location (Collision|BreakHitResult _outhit)) false false)
    (Default|EnableInteractions (Variables|/Game/FarmingSimulator/Core/GardeningComponents/Plants/BP_PlantParent.BP_PlantParent_C|GetBPC_InteractableComponent _plantactor) false)
    (bind _valid_ (CallFunction|ValidatePlacement))
    (Default|SetIsValid (Variables|/Game/FarmingSimulator/Core/GM_State_Farming.GM_State_Farming_C|GetPlantActor (Variables|Reference|GetGameState_Ref)) _valid_)))

(event Custom|PickUpTool
  ;[0.15 0.15 0.15 0.5] Picking up Hoe tool
  (CallFunction|PickUpToolServer (Variables|/Game/FarmingSimulator/Core/InteractionSystem/BPC_Interaction.BPC_Interaction_C|GetLastInteractionObject (Variables|/Game/ThirdPerson/Blueprints/BP_ThirdPersonCharacter.BP_ThirdPersonCharacter_C|GetBPC_Interaction (Variables|Reference|GetPlayerRef))) (.AsBP%20Third%20Person%20Character (Utilities|Casting|CastToBP_ThirdPersonCharacter (Game|GetPlayerCharacter 0)))))

(event Custom|SpawnPlant_Server
  (params (PlantActor :type BP%20Plant%20Parent%20Object%20Reference) (ActorTransform :type Transform))
  ;[0.15 0.15 0.15 0.5] Sow Plant For Cultivation
  (CallFunction|SpawnPantClient PlantActor ActorTransform))

(event Custom|SpawnPant_Client
  (params (Plant :type BP%20Plant%20Parent%20Object%20Reference) (SpawnTransform :type Transform))
  ;[0.15 0.15 0.15 0.5] Sow Plant For Cultivation
  (bind _returnvalue (Game|SpawnActorfromClass (Utilities|GetClass Plant) SpawnTransform "Undefined" "MultiplyWithRoot" 0 0))
  (Variables|Default|SetSpawnedPlantParent _returnvalue)
  (Utilities|FlowControl|Delay 0.2))

(event Custom|SpawnPlantActor_Server
  ;[0.15 0.15 0.15 0.5] Function to create and save actor reference
  (CallFunction|SpawnPlantActorClient))

(event Custom|SpawnPlantActor_Client
  ;[0.15 0.15 0.15 0.5] Function to create and save actor reference
  (bind _returnvalue (Game|SpawnActorfromClass "/Game/FarmingSimulator/Core/GardeningComponents/Plants/BP_Tomato.BP_Tomato_C" (Math|Transform|MakeTransform "0, 0, 0" "0, 0, 0" "1.000000,1.000000,1.000000") "Undefined" "MultiplyWithRoot" 0 0))
  (Variables|/Game/FarmingSimulator/Core/GM_State_Farming.GM_State_Farming_C|SetPlantActor (Variables|Reference|GetGameState_Ref) _returnvalue))

(event Custom|PickUpTool_Server
  (params (ToolInteractedWith :type Actor%20Object%20Reference) (OwnerPlayer :type BP%20Third%20Person%20Character%20Object%20Reference))
  ;[0.15 0.15 0.15 0.5] Picking up Hoe tool
  (Utilities|IsValid ToolInteractedWith
    (:Is%20Valid
      (Transformation|AttachComponentToComponent ToolInteractedWith (Variables|/Game/ThirdPerson/Blueprints/BP_ThirdPersonCharacter.BP_ThirdPersonCharacter_C|GetFarmingHoe OwnerPlayer) "None" "SnapToTarget" "SnapToTarget" "SnapToTarget" true))))

(event Custom|StartTilling_Client
  ;[0.15 0.15 0.15 0.5] Start Tilling
  (if (Variables|Default|GetToolEquipped?)
    (Animation|PlayAnimMontage (Variables|Reference|GetPlayerRef) "/Game/FarmingSimulator/AnimationRetargetting/Hoeing_Montage.Hoeing_Montage" 1.0 "None")
    (bind _asbp_item (Utilities|Casting|CastToBP_Item (Variables|Default|GetOverLappingActor%20ref)))
    (Class|BPIItems|OnAttackPressed(Message) _asbp_item)))

(event EventBeginPlay
  (bind _returnvalue (UserInterface|CreateWidget "/Game/FarmingSimulator/Widgets/WBP_ControlGuide.WBP_ControlGuide_C"))
  (Variables|Default|SetControllerGuid_Ref _returnvalue)
  (bind _asbp_third_person_character (Utilities|Casting|CastToBP_ThirdPersonCharacter (Game|GetPlayerCharacter 0)))
  (Utilities|IsValid _asbp_third_person_character
    (:Is%20Valid
      (Variables|Reference|SetPlayerRef _asbp_third_person_character)
      (bind _asgm_state_farming (Utilities|Casting|CastToGM_State_Farming (Game|GetGameState)))
      (Utilities|IsValid _asgm_state_farming
        (:Is%20Valid
          (Variables|Reference|SetGameState_Ref _asgm_state_farming)
          (Utilities|FlowControl|Delay 0.2)
          ;[0.15 0.15 0.15 0.5] Setting the plant object reference
          (CallFunction|SpawnPlantActorServer)
          (Default|StartPreviewing (Variables|/Game/FarmingSimulator/Core/GM_State_Farming.GM_State_Farming_C|GetPlantActor (Variables|Reference|GetGameState_Ref))))))))

(event EventTick
  (params (DeltaSeconds :type Float%20%28single-precision%29))
  ;[0.15 0.15 0.15 0.5] Spawning the plant preview where it can be placed
  (if (Variables|Default|GetStartPreview)
    (if (Variables|Default|GetHasSeed?)
      (Variables|/Game/FarmingSimulator/Core/GM_State_Farming.GM_State_Farming_C|GetPlantActor (Variables|Reference|GetGameState_Ref)
        (:then
          (CallFunction|MeshMovementTrace)
          (Rendering|SetActorHiddenInGame (Variables|/Game/FarmingSimulator/Core/GM_State_Farming.GM_State_Farming_C|GetPlantActor (Variables|Reference|GetGameState_Ref)) false))
        (:else)))))

(event Input|KeyboardEvents|1
  (params (Key :type Key%20Structure :default "None"))
  ;[0.15 0.15 0.15 0.5] Sheading/Drawing Tool
  (:Pressed
    (Default|DrawHoeServer (Variables|Reference|GetPlayerRef) (Variables|Default|GetToolEquipped?))))

(event Input|MouseEvents|LeftMouseButton
  (params (Key :type Key%20Structure :default "None"))
  (:Pressed
    (Default|StartTillingServer (.AsBP%20Third%20Person%20Character (Utilities|Casting|CastToBP_ThirdPersonCharacter (Game|GetPlayerCharacter 0))) (Variables|Default|GetToolEquipped?) (Variables|/Game/FarmingSimulator/Core/InteractionSystem/BPC_Interaction.BPC_Interaction_C|GetLastInteractionObject (Variables|/Game/ThirdPerson/Blueprints/BP_ThirdPersonCharacter.BP_ThirdPersonCharacter_C|GetBPC_Interaction (Variables|Reference|GetPlayerRef))))))

(event Input|KeyboardEvents|Tab
  (params (Key :type Key%20Structure :default "None"))
  ;[0.15 0.15 0.15 0.5] Inventory button
  (:Pressed
    (Game|Player|SetViewTargetwithBlend self (Variables|/Script/Engine.ChildActorComponent|GetChildActor (Variables|/Game/ThirdPerson/Blueprints/BP_ThirdPersonCharacter.BP_ThirdPersonCharacter_C|GetInventoryCamera (Variables|Reference|GetPlayerRef))) 0.5 "VTBlend_Linear" 0.0 false)
    (bind _returnvalue (UserInterface|CreateWidget "/Game/FarmingSimulator/Widgets/Inventory/WB_PlayerInventoryUI.WB_PlayerInventoryUI_C"))
    (UserInterface|Viewport|AddtoViewport _returnvalue 0)
    (Input|SetInputModeUIOnly self 0 "DoNotLock" false)
    (Variables|Default|SetbShowMouseCursor true)
    (Widget|SetVisibility (Variables|Default|GetControllerGuid_Ref) "Hidden")))

(event Input|KeyboardEvents|Q
  (params (Key :type Key%20Structure :default "None"))
  (bind _playerref (Variables|Reference|GetPlayerRef))
  (bind _plantingprogressbar (Variables|/Game/ThirdPerson/Blueprints/BP_ThirdPersonCharacter.BP_ThirdPersonCharacter_C|GetPlantingProgressBar _playerref))
  ;[0.15 0.15 0.15 0.5] Spawning the plant preview where it can be placed
  (:Pressed
    (Utilities|FlowControl|FlipFlop
      (:A
        (Variables|Default|SetStartPreview true)
        (Development|SetHiddeninGame _plantingprogressbar false false))
      (:B
        (Variables|Default|SetStartPreview false)
        (Rendering|SetActorHiddenInGame (Variables|/Game/FarmingSimulator/Core/GM_State_Farming.GM_State_Farming_C|GetPlantActor (Variables|Reference|GetGameState_Ref)) true)
        (Development|SetHiddeninGame _plantingprogressbar true false)))))

(event Input|KeyboardEvents|F
  (params (Key :type Key%20Structure :default "None"))
  (bind _gamestate_ref (Variables|Reference|GetGameState_Ref))
  (bind _plantactor (Variables|/Game/FarmingSimulator/Core/GM_State_Farming.GM_State_Farming_C|GetPlantActor _gamestate_ref))
  ;[0.15 0.15 0.15 0.5] Sow Plant For Cultivation
  (:Pressed
    (CallFunction|Sow _plantactor (Transformation|GetActorTransform _plantactor))))

(fn ConstructionScript)

(fn ValidatePlacement
  (for _array_element (Collision|GetOverlappingActors (Variables|/Game/FarmingSimulator/Core/GardeningComponents/Plants/BP_PlantParent.BP_PlantParent_C|GetValidationBox (Variables|/Game/FarmingSimulator/Core/GM_State_Farming.GM_State_Farming_C|GetPlantActor (Variables|Reference|GetGameState_Ref))) 0 :!class /Script/Engine.PrimitiveComponent)
    (if (!= (Utilities|GetClass _array_element) "/Game/FarmingSimulator/Core/GardeningComponents/BP_GardenPlace.BP_GardenPlace_C")
      (Utilities|Array|Add (LocalVariables|GetLocal_OverlappedActorsFiltered) _array_element)))
  (return (and (Utilities|Array|IsEmpty (LocalVariables|GetLocal_OverlappedActorsFiltered)) (not (Utilities|Array|IsEmpty (Collision|GetOverlappingActors (Variables|/Game/FarmingSimulator/Core/GardeningComponents/Plants/BP_PlantParent.BP_PlantParent_C|GetValidationBox (Variables|/Game/FarmingSimulator/Core/GM_State_Farming.GM_State_Farming_C|GetPlantActor (Variables|Reference|GetGameState_Ref))) "/Game/FarmingSimulator/Core/GardeningComponents/BP_GardenPlace.BP_GardenPlace_C" :!class /Script/Engine.PrimitiveComponent))))))

(fn Sow
  (params (PlantParent :type BP%20Plant%20Parent%20Object%20Reference) (ActorTransform :type Transform))
  (bind _spawnedplantparent (Variables|Default|GetSpawnedPlantParent))
  (Development|PrintString "Hello i am in sow plant function")
  (Utilities|IsValid PlantParent
    (:Is%20Valid
      (bind _valid_ (CallFunction|ValidatePlacement))
      (if _valid_
        (CallFunction|SpawnPlantServer PlantParent ActorTransform)
        (bind _asbp_garden_place (Utilities|Casting|CastToBP_GardenPlace (Utilities|Array|Get(acopy) (Collision|GetOverlappingActors _spawnedplantparent "/Game/FarmingSimulator/Core/GardeningComponents/BP_GardenPlace.BP_GardenPlace_C" :!class /Script/Engine.Actor))))
        (Default|AddPlant _asbp_garden_place _spawnedplantparent)
        (Default|Plant _spawnedplantparent)
        (else
          (Development|PrintString "Validation failed"))))
    (:Is%20Not%20Valid
      (Development|PrintString "Reference is not valid "))))

(fn UpdateWidgetPlantingProgress
  (params (Progress :type Float%20%28double-precision%29))
  (bind _aswb_plant_progress_bar (Utilities|Casting|CastToWB_PlantProgressBar (UserInterface|GetWidget (Variables|/Game/ThirdPerson/Blueprints/BP_ThirdPersonCharacter.BP_ThirdPersonCharacter_C|GetPlantingProgressBar (Variables|Reference|GetPlayerRef)))))
  (Utilities|IsValid _aswb_plant_progress_bar
    (:Is%20Valid
      (Variables|/Game/FarmingSimulator/Widgets/WB_PlantProgressBar.WB_PlantProgressBar_C|SetProgress _aswb_plant_progress_bar Progress))))

(fn SpendMoney
  (params (Money :type Integer))
  (bind _gamestate_ref (Variables|Reference|GetGameState_Ref))
  (bind _output_get (Variables|/Game/FarmingSimulator/Core/GM_State_Farming.GM_State_Farming_C|SetMoney _gamestate_ref (- (Variables|/Game/FarmingSimulator/Core/GM_State_Farming.GM_State_Farming_C|GetMoney _gamestate_ref) Money)))
  (return _output_get))