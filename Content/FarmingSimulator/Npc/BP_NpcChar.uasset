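; BP_NpcChar is a farming simulator NPC that patrols a looping route of destination actors.
; On BeginPlay, if its States enum holds one particular value, it uses AI MoveTo toward the current entry in the Destinations array.
; Each successful arrival triggers a short delay, then advances the Target index, wrapping to the start, and moves again.
; Failed moves have no handler, so the patrol stops there.
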(event EventBeginPlay
  (if (Utilities|Enum|Equal(Enum) (Variables|Default|GetStates) "NewEnumerator1")
    (AI|AIMoveTo self "0, 0, 0" (Utilities|Array|Get(acopy) (Variables|Default|GetDestinations) (Variables|Default|GetTarget)) 5.0 false :!label _label
      (:OnSuccess
        (Utilities|FlowControl|Delay 1.0)
        (if (== (+ (Variables|Default|GetTarget) 1) (Utilities|Array|Length (Variables|Default|GetDestinations)))
          (Variables|Default|SetTarget 0)
          (goto _label)
          (else
            (Variables|Default|SetTarget (+ (Variables|Default|GetTarget) 1))
            (goto _label)))))))

(fn ConstructionScript)